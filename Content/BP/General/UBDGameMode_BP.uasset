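; Game mode for a dedicated-server match that runs the lobby, game start and server shutdown.
; On login it asks ServerRequest whether the player is allowed, returning rejected players to the main menu.
; Player counts trigger a delayed or immediate start, which teleports pawns from tagged wait-room starts to shuffled game spawns without map travel.
; It reports status changes through ServerRequest and uses timers and logout counts to close empty servers.
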(event Custom|StartGame
  (Utilities|FlowControl|DoOnce false
    (:Completed
      (Utilities|Time|ClearandInvalidateTimerbyHandle (Variables|Default|GetWaitTimer))
      (Class|ServerRequestComponent|ChangeServerStatus (Variables|Default|GetServerRequest) "Starting" (Variables|Default|GetServerId))
      (Variables|/Game/BP/General/UBD_GS.UBD_GS_C|SetGameState (Variables|Default|GetAs%20UBD%20GS) "NewEnumerator1")
      (bind _outactors (Actor|GetAllActorsOfClass (Variables|Default|GetPlayerControllerClass)))
      (for _array_element _outactors
        (Class|GameStateI|StartGameTimer(Message) _array_element))
      (Development|PrintString "StartingGame")
      (bind _returnvalue (Utilities|Time|SetTimerbyEvent (delegate Custom|LoadMap) (Variables|Default|GetBeforeStartTimer)))
      (Variables|Default|SetStartTimer _returnvalue))))

(event Custom|LoadMap
  (Variables|Default|SetGameStarted true)
  (bind _outactors (Actor|GetAllActorsOfClass (Variables|Default|GetDefaultPawnClass)))
  (for _array_element _outactors
    (bind _returnvalue (CallFunction|GetGameplayStartTransform))
    (Transformation|SetActorTransform _array_element _returnvalue))
  (bind _outactors_2 (Actor|GetAllActorsOfClass (Variables|Default|GetPlayerControllerClass)))
  (for _array_element_2 _outactors_2
    (Class|GameStateI|GameStart(Message) _array_element_2))
  (Variables|/Game/BP/General/UBD_GS.UBD_GS_C|SetGameState (Variables|Default|GetAs%20UBD%20GS) "NewEnumerator2")
  (Class|ServerRequestComponent|ChangeServerStatus (Variables|Default|GetServerRequest) "Ingame" (Variables|Default|GetServerId)))

(event Custom|StartGameAfterWaitMore
  (Utilities|FlowControl|DoOnce false
    (:Completed
      (bind _returnvalue (Utilities|Time|SetTimerbyEvent (delegate Custom|StartGame) 3e+02))
      (Variables|Default|SetWaitTimer _returnvalue)
      (Utilities|Time|ClearandInvalidateTimerbyHandle (Variables|Default|GetShutDonwTimer)))))

(event Custom|ShutdownServer
  (bind _returnvalue (Class|UBDFunctionLibrary|IsEditor))
  (if (not _returnvalue)
    (if (Networking|IsDedicatedServer)
      (Class|UBDFunctionLibrary|RequestExitServer false))))

(event Custom|ShutDownTimerStart
  (bind _returnvalue (Utilities|Time|SetTimerbyEvent (delegate Custom|ShutdownServer) 3e+02))
  (Variables|Default|SetShutDonwTimer _returnvalue))

(event Custom|OnPlayerCheckRequest
  (params (Allowed :type Boolean) (PlayerId :type Integer) (Abiliity1 :type String) (Ability2 :type String) (Ability3 :type String))
  (bind _players (Variables|Default|GetPlayers))
  (bind _playerscount (Variables|Default|GetPlayersCount))
  (bind (_value _returnvalue) (Utilities|Map|Find _players PlayerId))
  (if Allowed
    (switch Utilities|FlowControl|Switch|SwitchonGameState (Variables|/Game/BP/General/UBD_GS.UBD_GS_C|GetGameState (Variables|Default|GetAs%20UBD%20GS))
      (:NewEnumerator0
        (bind _asbp_top_down_player_controller (Utilities|Casting|CastToBP_TopDownPlayerController _value))
        (Default|SetinGameStatus _asbp_top_down_player_controller)
        (bind _result (Math|Integer|IncrementInt _playerscount)
          (:%20%20
            (if (>= _playerscount (Variables|Default|GetMinPlayerCount))
              (CallFunction|StartGameAfterWaitMore))
            (if (== _result (Variables|Default|GetMaxPlayerCount))
              (CallFunction|StartGame)))))
      (:NewEnumerator1
        ;[1 1 1] If he allowed stop shutdown if not kick him out
        (Development|PrintString "CheckIfHeAllowedToPlay" :!label _label)
        (Utilities|Time|ClearandInvalidateTimerbyHandle (Variables|Default|GetShutDonwTimer)))
      (:NewEnumerator2
        (goto _label))
      (:NewEnumerator3
        (CallFunction|Kick _value :!label _label_2)))
    (else
      (Utilities|Array|Add (Variables|Default|GetBannedPlayers) PlayerId)
      (if _returnvalue
        (goto _label_2)))))

(event Custom|Kick
  (params (PlayerController :type Player%20Controller%20Object%20Reference))
  (bind _asbp_top_down_player_controller (Utilities|Casting|CastToBP_TopDownPlayerController PlayerController))
  (Default|GoMainMenu _asbp_top_down_player_controller))

(event EventBeginPlay
  (|CallParentFunction)
  (EventDispatchers|AssignOnCheckPlayerResult (Variables|Default|GetServerRequest) (EventDispatchers|CreateEvent :!event Custom|OnPlayerCheckRequest))
  (bind _returnvalue (Class|UBDFunctionLibrary|GetServerId))
  (Variables|Default|SetServerId _returnvalue)
  (bind _asubd_gs (Utilities|Casting|CastToUBD_GS (Game|GetGameState))
    (:then
      (Variables|Default|SetAs%20UBD%20GS _asubd_gs))
    (:CastFailed
      _))
  (bind _returnvalue_2 (Utilities|GetDataTableRow "/Game/Data/PlayerStarts_DT.PlayerStarts_DT" "WaitRoom")
    (:then
      (Variables|Default|SetWaitRoomTag (Utilities|Struct|BreakPlayerStartStructure _returnvalue_2)))
    (:RowNotFound
      _))
  (bind _returnvalue_3 (Utilities|GetDataTableRow "/Game/Data/PlayerStarts_DT.PlayerStarts_DT" "GameSpawn")
    (:then
      (Variables|Default|SetPlaySpawnTags (Utilities|Struct|BreakPlayerStartStructure _returnvalue_3)))
    (:RowNotFound
      _))
  (CallFunction|GetWaitRoomPlayerStart)
  (CallFunction|ShutDownTimerStart))

(event EventDestroyed
  (if (Networking|IsDedicatedServer)
    (bind _returnvalue (Class|UBDFunctionLibrary|GetServerId))
    (Class|ServerRequestComponent|ChangeServerStatus (Variables|Default|GetServerRequest) "Finishing" _returnvalue))
  (|CallParentFunction))

(event EventPostLogin
  (params (NewPlayer :type Player%20Controller%20Object%20Reference))
  (|CallParentFunction NewPlayer)
  (bind _asubdplayer_state_bp (Utilities|Casting|CastToUBDPlayerState_BP (Variables|/Script/Engine.Controller|GetPlayerState NewPlayer)))
  (Utilities|Map|Add (Variables|Default|GetPlayers) (Variables|/Game/BP/TopDown/Blueprints/UBDPlayerState_BP.UBDPlayerState_BP_C|GetPlayerAuthID _asubdplayer_state_bp) NewPlayer)
  (if (!= (Utilities|Array|FindItem (Variables|Default|GetBannedPlayers) (Variables|/Game/BP/TopDown/Blueprints/UBDPlayerState_BP.UBDPlayerState_BP_C|GetPlayerAuthID _asubdplayer_state_bp)) -1)
    (CallFunction|Kick NewPlayer)
    (else
      (Class|ServerRequestComponent|IsPlayerAllowed (Variables|Default|GetServerRequest) (Variables|/Game/BP/TopDown/Blueprints/UBDPlayerState_BP.UBDPlayerState_BP_C|GetPlayerAuthID _asubdplayer_state_bp) (Variables|Default|GetServerId)))))

(event EventOnLogout
  (params (ExitingController :type Controller%20Object%20Reference))
  (|CallParentFunction ExitingController)
  (bind _result (Math|Integer|DecrementInt (Variables|Default|GetPlayersCount))
    (:%20%20
      (if (<= _result 0)
        (switch Utilities|FlowControl|Switch|SwitchonGameState (Variables|/Game/BP/General/UBD_GS.UBD_GS_C|GetGameState (Variables|Default|GetAs%20UBD%20GS))
          (:NewEnumerator0
            (CallFunction|ShutdownServer :!label _label))
          (:NewEnumerator1
            (goto _label))
          (:NewEnumerator2
            (CallFunction|ShutDownTimerStart))
          (:NewEnumerator3
            (goto _label)))))))

(fn ConstructionScript)

(fn ChoosePlayerStart
  (params (Player :type Controller%20Object%20Reference))
  (bind _possiblewaitroomstarts (Variables|Default|GetPossibleWaitRoomStarts))
  (bind _gamestarted (Variables|Default|GetGameStarted))
  (bind _possiblegamestart (Variables|Default|GetPossibleGameStart))
  (bind _returnvalue (select _gamestarted _possiblegamestart _possiblewaitroomstarts))
  (if (Utilities|Array|IsNotEmpty (select (Variables|Default|GetGameStarted) (Variables|Default|GetPossibleGameStart) (Variables|Default|GetPossibleWaitRoomStarts)))
    _
    (elif (Variables|Default|GetGameStarted)
      (CallFunction|GetPlaySpawnStarts)
      (else
        (CallFunction|GetWaitRoomPlayerStart))))
  (bind _output_get (LocalVariables|SetStart (Utilities|Array|Get(acopy) _returnvalue)))
  (Utilities|Array|RemoveItem _returnvalue _output_get)
  (Utilities|IsValid (LocalVariables|GetStart)
    (:Is%20Valid
      (return (LocalVariables|GetStart)))
    (:Is%20Not%20Valid
      (bind _returnvalue_2 (|CallParentFunction Player))
      (return _returnvalue_2))))

(fn GetWaitRoomPlayerStart
  (bind _outactors (Actor|GetAllActorsOfClasswithTag (Variables|Default|GetPlayerStartClass) (Variables|Default|GetWaitRoomTag)))
  (bind _output_get (Variables|Default|SetPossibleWaitRoomStarts _outactors))
  (Utilities|Array|Shuffle _output_get))

(fn GetPlaySpawnStarts
  (bind _outactors (Actor|GetAllActorsOfClasswithTag (Variables|Default|GetPlayerStartClass) (Variables|Default|GetPlaySpawnTags)))
  (bind _output_get (Variables|Default|SetPossibleGameStart _outactors))
  (Utilities|Array|Shuffle _output_get))

(fn GetGameplayStartTransform
  (if (Utilities|Array|IsNotEmpty (Variables|Default|GetPossibleGameStart))
    _
    (else
      (CallFunction|GetPlaySpawnStarts)))
  (bind _output_get (LocalVariables|SetStart (Utilities|Array|Get(acopy) (Variables|Default|GetPossibleGameStart))))
  (Utilities|Array|RemoveItem (Variables|Default|GetPossibleGameStart) _output_get)
  (return (Transformation|GetActorTransform (LocalVariables|GetStart))))