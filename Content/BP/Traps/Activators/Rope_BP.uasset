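; Rope trap activator that triggers its linked traps while characters stand inside its box trigger.
; Tracks overlapping characters in an array, so the first to enter sends an interact request to each entry in TrapsToActivate and the last to leave sends a stop request.
; The Cube mesh drops slightly while triggered and returns to its origin on release.
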(event OnComponentBeginOverlap(Box)
  (params (OverlappedComponent :type Primitive%20Component%20Object%20Reference) (OtherActor :type Actor%20Object%20Reference) (OtherComp :type Primitive%20Component%20Object%20Reference) (OtherBodyIndex :type Integer) (bFromSweep :type Boolean) (SweepResult :type Hit%20Result%20Structure%20%28by%20ref%29))
  ;[1 1 1] TODO DO
  (bind _ascharacter (Utilities|Casting|CastToCharacter OtherActor))
  (bind _returnvalue (Utilities|Array|Add (Variables|Default|GetOverlapedActors) _ascharacter))
  (if (== _returnvalue 0)
    (for _array_element (Variables|Default|GetTrapsToActivate)
      (Class|InteractI|InteractRequest(Message) _array_element))
    (Transformation|SetRelativeLocation (Variables|Default|GetCube) "0.000000,0.000000,-5.000000" false false)))

(event OnComponentEndOverlap(Box)
  (params (OverlappedComponent :type Primitive%20Component%20Object%20Reference) (OtherActor :type Actor%20Object%20Reference) (OtherComp :type Primitive%20Component%20Object%20Reference) (OtherBodyIndex :type Integer))
  ;[1 1 1] TODO DO
  (bind _ascharacter (Utilities|Casting|CastToCharacter OtherActor))
  (bind _returnvalue (Utilities|Array|RemoveItem (Variables|Default|GetOverlapedActors) _ascharacter))
  (if _returnvalue
    (if (Utilities|Array|IsEmpty (Variables|Default|GetOverlapedActors))
      (for _array_element (Variables|Default|GetTrapsToActivate)
        (Class|InteractI|StopInteractRequest(Message) _array_element))
      (Transformation|SetRelativeLocation (Variables|Default|GetCube) "0, 0, 0" false false))))

(fn ConstructionScript)