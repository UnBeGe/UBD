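; Pressure plate trap activator that triggers its linked traps while Characters stand on it.
; Box overlap events track occupants in an array, so only the first arrival activates and the last departure deactivates.
; TrapsToActivate receive interact and stop-interact messages, while the Cube sinks slightly based on its bounds and plays BladeSound on activation, then resets when empty.
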(event OnComponentBeginOverlap(Box)
  (params (OverlappedComponent :type Primitive%20Component%20Object%20Reference) (OtherActor :type Actor%20Object%20Reference) (OtherComp :type Primitive%20Component%20Object%20Reference) (OtherBodyIndex :type Integer) (bFromSweep :type Boolean) (SweepResult :type Hit%20Result%20Structure%20%28by%20ref%29))
  (CallFunction|ActivateTrap OtherActor))

(event OnComponentEndOverlap(Box)
  (params (OverlappedComponent :type Primitive%20Component%20Object%20Reference) (OtherActor :type Actor%20Object%20Reference) (OtherComp :type Primitive%20Component%20Object%20Reference) (OtherBodyIndex :type Integer))
  (CallFunction|DeactivateTrap OtherActor))

(event Custom|ActivateTrap
  (params (Object :type Object%20Object%20Reference))
  (bind _cube (Variables|Default|GetCube))
  (bind _ascharacter (Utilities|Casting|CastToCharacter Object))
  (bind _returnvalue (Utilities|Array|Add (Variables|Default|GetOverlapedActors) _ascharacter))
  (if (== _returnvalue 0)
    (for _array_element (Variables|Default|GetTrapsToActivate)
      (Class|InteractI|InteractRequest(Message) _array_element))
    (Transformation|SetRelativeLocation _cube (Math|Vector|MakeVector 0.0 0.0 (* (* (.Z (Math|Vector|BreakVector (.BoxExtent (Collision|GetComponentBounds _cube)))) 0.2) -1.0)) false false)
    (Audio|Components|Audio|Play (Variables|Default|GetBladeSound) 0.0)))

(event Custom|DeactivateTrap
  (params (Object :type Object%20Object%20Reference))
  (bind _ascharacter (Utilities|Casting|CastToCharacter Object))
  (bind _returnvalue (Utilities|Array|RemoveItem (Variables|Default|GetOverlapedActors) _ascharacter))
  (if _returnvalue
    (if (Utilities|Array|IsEmpty (Variables|Default|GetOverlapedActors))
      (for _array_element (Variables|Default|GetTrapsToActivate)
        (Class|InteractI|StopInteractRequest(Message) _array_element))
      (Transformation|SetRelativeLocation (Variables|Default|GetCube) "0, 0, 0" false false))))

(event EventBeginPlay)

(event Collision|EventActorBeginOverlap
  (params (OtherActor :type Actor%20Object%20Reference)))

(event EventTick
  (params (DeltaSeconds :type Float%20%28single-precision%29)))

(fn ConstructionScript)