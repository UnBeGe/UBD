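; Base enemy that equips a weapon and picks a player to chase.
; On BeginPlay the server reads a Weapons data table row, async-loads and spawns the weapon actor, and passes it the enemy's Ability System Component.
; The ActiveWeapon RepNotify attaches it to the mesh and links its async-loaded animation layer.
; Sphere overlap or player damage sets a living player as the Blackboard target unless one is already valid.
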(event OnComponentBeginOverlap(Sphere)
  (params (OverlappedComponent :type Primitive%20Component%20Object%20Reference) (OtherActor :type Actor%20Object%20Reference) (OtherComp :type Primitive%20Component%20Object%20Reference) (OtherBodyIndex :type Integer) (bFromSweep :type Boolean) (SweepResult :type Hit%20Result%20Structure%20%28by%20ref%29))
  (bind _asbp_top_down_character (Utilities|Casting|CastToBP_TopDownCharacter OtherActor))
  (CallFunction|DecidetoChace _asbp_top_down_character))

(event Custom|SetNewWeapon
  (params (ActiveWeaponItem :type Base%20Item%20Structure))
  (bind _activeweapon (Variables|Default|GetActiveWeapon))
  ;[1 1 1] WaponManagment
  (Utilities|IsValid _activeweapon
    (:Is%20Valid
      (Actor|DestroyActor _activeweapon)
      (Class|InventoryComponent|AddItem (Variables|Default|GetInventory) (Variables|Default|GetActiveWeaponItem)))
    (:Is%20Not%20Valid
      _))
  (Variables|Default|SetActiveWeaponItem ActiveWeaponItem)
  (CallFunction|SpawnWeapon))

(event Custom|SpawnWeapon
  (bind _self self)
  ;[1 1 1] WaponManagment
  (Variables|Default|SetActiveWeapon 0)
  (bind _class (Utilities|AsyncLoadClassAsset (.ActorReference (Utilities|Struct|BreakBaseItem (Variables|Default|GetActiveWeaponItem))))
    (:Completed
      (bind _asbase_weapon (Utilities|Casting|CastToBaseWeaponClass _class))
      (bind _returnvalue (Game|SpawnActorfromClass _asbase_weapon (Math|Transform|MakeTransform "0, 0, 0" "0, 0, 0" "1.000000,1.000000,1.000000") "Undefined" "MultiplyWithRoot" _self 0))
      (bind _output_get (Variables|Default|SetActiveWeapon _returnvalue))
      (Variables|/Game/BP/TopDown/Blueprints/Weapons/BaseWeapon.BaseWeapon_C|SetASC _output_get (Ability|GetAbilitySystemComponent _self)))))

(event Custom|WeaponUpdate
  (bind _activeweapon (Variables|Default|GetActiveWeapon))
  (bind _mesh (Variables|Character|GetMesh))
  ;[1 1 1] WaponManagment
  (Utilities|IsValid _activeweapon
    (:Is%20Valid
      (Transformation|AttachComponentToComponent _activeweapon (Variables|Character|GetMesh) (Variables|/Game/BP/TopDown/Blueprints/Weapons/BaseWeapon.BaseWeapon_C|GetSocketName _activeweapon) "SnapToTarget" "SnapToTarget" "SnapToTarget" true)
      ;;[1 1 1] Probably spike
      (bind _class (Utilities|AsyncLoadClassAsset (Variables|/Game/BP/TopDown/Blueprints/Weapons/BaseWeapon.BaseWeapon_C|GetAnimLayerClass _activeweapon))
        (:Completed
          (bind _asanim_instance (Utilities|Casting|CastToAnimInstanceClass _class))
          (Class|SkeletalMeshComponent|UnlinkAnimClassLayers _mesh (Variables|Default|GetCurrentLayer))
          (Components|SkeletalMesh|AnimationBlueprintLinking|LinkAnimClassLayers _mesh _asanim_instance)
          (Variables|Default|SetCurrentLayer _asanim_instance))))))

(event Custom|DecideToChace
  (params (InputPin :type BP%20Top%20Down%20Character%20Object%20Reference))
  (bind _returnvalue (AI|GetBlackboard 0))
  (Utilities|IsValid (Variables|Default|GetChasingPlayer)
    (:Is%20Not%20Valid
      (if (Class|UBDCharacter|IsAlive InputPin)
        (Variables|Default|SetChasingPlayer InputPin)
        (Utilities|IsValid (Variables|Default|GetChasingPlayer)
          (:Is%20Valid
            (Utilities|IsValid _returnvalue
              (:Is%20Valid
                (AI|Components|Blackboard|SetValueasObject _returnvalue (Variables|Default|GetPlayerKeyName) (Variables|Default|GetChasingPlayer))))))))))

(event Custom|DamagedBy_1
  (params (DamageCaller :type Actor%20Object%20Reference))
  (bind _asbp_top_down_character (Utilities|Casting|CastToBP_TopDownCharacter DamageCaller))
  (CallFunction|DecidetoChace _asbp_top_down_character))

(event EventBeginPlay
  (Networking|SwitchHasAuthority
    (:Authority
      (Variables|Default|SetSavedStartLocation (Transformation|GetActorLocation))
      (bind _returnvalue (Utilities|GetDataTableRow "/Game/Data/Items/Weapons.Weapons" "BigSword")
        (:then
          (CallFunction|SetNewWeapon _returnvalue))))))

(fn ConstructionScript)

(fn OnRepActiveWeapon
  (CallFunction|WeaponUpdate))